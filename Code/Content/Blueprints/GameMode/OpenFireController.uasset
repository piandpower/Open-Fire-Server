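; OpenFireController is a controller for OpenFirePawn that keeps the pawn locked to its airplane.
; On BeginPlay it casts the controlled pawn to OpenFirePawn and stores the reference.
; Each Tick, while the pawn's Airplane is valid, it copies the airplane's location, rotation and scale onto the pawn without sweeping.
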(event EventBeginPlay
  (bind _asopen_fire_pawn (Utilities|Casting|CastToOpenFirePawn (Pawn|GetControlledPawn)))
  (Variables|Default|SetOpenFirePawn _asopen_fire_pawn))

(event EventTick
  (params (DeltaSeconds :type Float%20%28single-precision%29))
  (bind _openfirepawn (Variables|Default|GetOpenFirePawn))
  (bind _airplane (Variables|/Game/Blueprints/GameMode/OpenFirePawn.OpenFirePawn_C|GetAirplane _openfirepawn))
  (bind _returnvalue (Transformation|GetActorTransform _airplane))
  (bind (_location _rotation _scale) (Math|Transform|BreakTransform _returnvalue))
  (Utilities|IsValid (Variables|/Game/Blueprints/GameMode/OpenFirePawn.OpenFirePawn_C|GetAirplane (Variables|Default|GetOpenFirePawn))
    (:Is%20Valid
      (Transformation|SetActorTransform _openfirepawn (Math|Transform|MakeTransform _location _rotation _scale)))))

(fn ConstructionScript)