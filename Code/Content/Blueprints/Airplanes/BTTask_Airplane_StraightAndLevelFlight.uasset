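; Behavior Tree task that steers an AI-controlled B_Airplane back to straight and level flight.
; Each tick it zeroes yaw input and levels roll first, then pitch, using proportional input that saturates outside a small angle band.
; Once both axes are within tolerance, it finishes successfully after a short delay.
; It also draws a debug sphere at the plane and reads a blackboard target that it never uses.
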(event EventTick
  (params (OwnerActor :type Actor%20Object%20Reference) (DeltaSeconds :type Float%20%28single-precision%29))
  (bind _airplane (Variables|Default|GetAirplane))
  (bind _returnvalue (Transformation|GetActorRotation _airplane))
  (bind (_pitch _yaw _roll) (Class|KismetMathLibrary|BreakRot _returnvalue))
  (Rendering|Debug|DrawDebugSphere (Transformation|GetActorLocation (Variables|Default|GetAirplane)) 1e+02 12 "(R=1.000000,G=0.500000,B=1.000000,A=1.000000)" 0.0)
  (Default|Yaw (Variables|Default|GetAirplane) 0.0)
  (bind _stable (CallFunction|SetRoll _roll))
  (if _stable
    (bind _stable_2 (CallFunction|SetPitch _pitch))
    (if _stable_2
      (Utilities|FlowControl|Delay 1.0)
      (AI|BehaviorTree|FinishExecute true))
    (else
      (Default|Pitch (Variables|Default|GetAirplane) 0.0))))

(event EventReceiveExecute
  (params (OwnerActor :type Actor%20Object%20Reference))
  (bind _ascontroller (Utilities|Casting|CastToController OwnerActor))
  (bind _asb_airplane (Utilities|Casting|CastToB_Airplane (Pawn|GetControlledPawn _ascontroller)))
  (Variables|Default|SetAirplane _asb_airplane)
  (Variables|Default|SetTarget (AI|BehaviorTree|GetBlackboardValueasActor (Variables|Default|GetTargetKey))))

(fn SetRoll
  (params (Roll :type Float%20%28single-precision%29 :default 0.0))
  (bind _returnvalue (Math|Float|Absolute(Float) Roll))
  (bind _returnvalue_2 (< _returnvalue 1e+01))
  (if _returnvalue_2
    (LocalVariables|SetDesire (* _returnvalue 0.1))
    (else
      (LocalVariables|SetDesire 1.0)))
  (if (< Roll 0.0)
    (Default|Roll (Variables|Default|GetAirplane) (LocalVariables|GetDesire))
    (else
      (Default|Roll (Variables|Default|GetAirplane) (- 0.0 (LocalVariables|GetDesire)))))
  (return _returnvalue_2))

(fn SetPitch
  (params (Pitch :type Float%20%28single-precision%29 :default 0.0))
  (bind _returnvalue (Math|Float|Absolute(Float) Pitch))
  (bind _returnvalue_2 (< _returnvalue 1e+01))
  (if _returnvalue_2
    (LocalVariables|SetDesire (* _returnvalue 0.1))
    (else
      (LocalVariables|SetDesire 1.0)))
  (if (< Pitch 0.0)
    (Default|Pitch (Variables|Default|GetAirplane) (- 0.0 (LocalVariables|GetDesire)))
    (else
      (Default|Pitch (Variables|Default|GetAirplane) (LocalVariables|GetDesire))))
  (return _returnvalue_2))