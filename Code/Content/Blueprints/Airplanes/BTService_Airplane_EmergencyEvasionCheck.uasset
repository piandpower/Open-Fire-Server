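; Behavior tree service that checks whether an AI-controlled airplane needs emergency evasion from an obstacle ahead.
; Each tick it line-traces on the Visibility channel along the pawn's forward vector and writes the result to the emergency evasion Blackboard flag.
; On a hit it stores the hit normal as the obstacle up vector and draws debug lines to the impact and along its normal.
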(event EventTick
  (params (OwnerActor :type Actor%20Object%20Reference) (DeltaSeconds :type Float%20%28single-precision%29))
  (bind _returnvalue (AI|GetAIController OwnerActor))
  (bind (_outhit _returnvalue_2) (Collision|LineTraceByChannel (Transformation|GetActorLocation (Pawn|GetControlledPawn _returnvalue)) (+ (Transformation|GetActorLocation (Pawn|GetControlledPawn _returnvalue)) (* (Transformation|GetActorForwardVector (Pawn|GetControlledPawn _returnvalue)) 5e+03)) "TraceTypeQuery1" false 0 "None"))
  (Class|BTFunctionLibrary|SetBlackboardValueasBool (Variables|Default|GetEmegencyEvasionKey) _returnvalue_2)
  (if _returnvalue_2
    (AI|BehaviorTree|SetBlackboardValueasVector (Variables|Default|GetObstacleUpVectorKey) (.Normal (Collision|BreakHitResult _outhit)))
    (CallFunction|DebugDrawCustom (Transformation|GetActorLocation (Pawn|GetControlledPawn _returnvalue)) (.Location (Collision|BreakHitResult _outhit)) (.ImpactNormal (Collision|BreakHitResult _outhit)))))

(fn DebugDrawCustom
  (params (AirplaneLocation :type Vector :default "0, 0, 0") (HitLocation :type Vector :default "0, 0, 0") (HitNormal :type Vector :default "0, 0, 0"))
  (Rendering|Debug|DrawDebugLine AirplaneLocation HitLocation "(R=1.000000,G=0.500000,B=0.000000,A=1.000000)" 3.0 3.0)
  (Rendering|Debug|DrawDebugLine HitLocation (+ HitLocation (* HitNormal 1e+02)) "(R=1.000000,G=0.200000,B=0.000000,A=1.000000)" 3.0 1e+01))