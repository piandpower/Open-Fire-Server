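; Behavior tree task that makes an AI-controlled B_Airplane perform a "cobra maneuver", implemented as a sustained full-pitch loop.
; On execute it caches the airplane and its starting forward vector, plus a blackboard target that goes unused.
; Each tick it applies constant pitch with zero yaw and roll and draws a debug sphere.
; It finishes successfully once the heading has left and then returned to within a small angle of the start.
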(event EventTick
  (params (OwnerActor :type Actor%20Object%20Reference) (DeltaSeconds :type Float%20%28single-precision%29))
  (if (< (Class|KismetMathLibrary|DegAcos (Math|Vector|DotProduct (Variables|Default|GetForwardVector) (Transformation|GetActorForwardVector (Variables|Default|GetAirplane)))) 1e+01)
    (if (Variables|Default|GetStartManeuver)
      (AI|BehaviorTree|FinishExecute true)
      (else
        (CallFunction|CobraManeuver :!label _label)
        (Rendering|Debug|DrawDebugSphere (Transformation|GetActorLocation (Variables|Default|GetAirplane)) 1e+02 12 "(R=1.000000,G=0.000000,B=1.000000,A=1.000000)" 0.0)))
    (else
      (Variables|Default|SetStartManeuver true)
      (goto _label))))

(event EventReceiveExecute
  (params (OwnerActor :type Actor%20Object%20Reference))
  (bind _ascontroller (Utilities|Casting|CastToController OwnerActor))
  (bind _asb_airplane (Utilities|Casting|CastToB_Airplane (Pawn|GetControlledPawn _ascontroller)))
  (Variables|Default|SetAirplane _asb_airplane)
  (Variables|Default|SetTarget (AI|BehaviorTree|GetBlackboardValueasActor (Variables|Default|GetTargetKey)))
  (Variables|Default|SetForwardVector (Transformation|GetActorForwardVector (Variables|Default|GetAirplane)))
  (Variables|Default|SetStartManeuver false))

(fn CobraManeuver
  (Default|Pitch (Variables|Default|GetAirplane) -2.0)
  (Default|Yaw (Variables|Default|GetAirplane) 0.0)
  (Default|Roll (Variables|Default|GetAirplane) 0.0))