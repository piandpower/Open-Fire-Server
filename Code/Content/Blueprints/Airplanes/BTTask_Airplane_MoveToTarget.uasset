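; Behavior tree task that steers an AI-controlled B_Airplane toward a blackboard target actor.
; On execute it caches the pawn and target, taking the view angle from the blackboard or defaulting to 180 degrees.
; Each tick, while the target is in view, it feeds the relative vector into SetRotationSpeed and draws a debug sphere at the airplane.
; The task fails when the target leaves view and has no success exit.
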(event EventTick
  (params (OwnerActor :type Actor%20Object%20Reference) (DeltaSeconds :type Float%20%28single-precision%29))
  (bind _view (CallFunction|IsView (Variables|Default|GetAirplane) (Variables|Default|GetTarget) (Variables|Default|GetViiewAngle)))
  (if _view
    (bind _relativevector (CallFunction|GetRelativeVector (Variables|Default|GetTarget) (Variables|Default|GetAirplane)))
    (CallFunction|SetRotationSpeed _relativevector "0, 0, 0" (Variables|Default|GetAirplane))
    (Rendering|Debug|DrawDebugSphere (Transformation|GetActorLocation (Variables|Default|GetAirplane)) 1e+02 12 "(R=0.000000,G=1.000000,B=0.000000,A=1.000000)" 0.0)
    (else
      (AI|BehaviorTree|FinishExecute false))))

(event EventReceiveExecute
  (params (OwnerActor :type Actor%20Object%20Reference))
  (bind _ascontroller (Utilities|Casting|CastToController OwnerActor))
  (bind _asb_airplane (Utilities|Casting|CastToB_Airplane (Pawn|GetControlledPawn _ascontroller)))
  (Variables|Default|SetAirplane _asb_airplane)
  (Variables|Default|SetTarget (AI|BehaviorTree|GetBlackboardValueasActor (Variables|Default|GetTargetKey)))
  (if (Variables|Default|GetUseViewAngle)
    (Variables|Default|SetViiewAngle (Class|BTFunctionLibrary|GetBlackboardValueasFloat (Variables|Default|GetViewAngleKey)))
    (else
      (Variables|Default|SetViiewAngle 1.8e+02))))