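; Behavior tree task that pitches an AI-controlled airplane in an emergency evasion from an obstacle.
; On execute it caches the controlled B_Airplane and the obstacle's up vector from the blackboard, or finishes successfully if the evasion flag is off.
; Each tick draws a debug sphere, zeroes roll and yaw, and applies constant negative pitch.
; It fails only if the angle between up vectors drops below zero, which arccosine never returns.
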(event EventReceiveExecute
  (params (OwnerActor :type Actor%20Object%20Reference))
  (if (Class|BTFunctionLibrary|GetBlackboardValueasBool (Variables|Default|GetEmergencyEvasionKey))
    (bind _ascontroller (Utilities|Casting|CastToController OwnerActor))
    (bind _asb_airplane (Utilities|Casting|CastToB_Airplane (Pawn|GetControlledPawn _ascontroller)))
    (Variables|Default|SetAirplane _asb_airplane)
    (Variables|Default|SetObstacleUpVector (Class|BTFunctionLibrary|GetBlackboardValueasVector (Variables|Default|GetObstacleUpVectorKey)))
    (else
      (AI|BehaviorTree|FinishExecute true))))

(event EventTick
  (params (OwnerActor :type Actor%20Object%20Reference) (DeltaSeconds :type Float%20%28single-precision%29))
  (bind _airplane (Variables|Default|GetAirplane))
  (Rendering|Debug|DrawDebugSphere (Transformation|GetActorLocation (Variables|Default|GetAirplane)) 1e+02 12 "(R=0.000000,G=1.000000,B=1.000000,A=1.000000)" 0.0)
  (Default|Roll _airplane 0.0)
  (Default|Yaw _airplane 0.0)
  (if (< (Class|KismetMathLibrary|DegAcos (Math|Vector|DotProduct (Variables|Default|GetObstacleUpVector) (Transformation|GetActorUpVector (Variables|Default|GetAirplane)))) 0.0)
    (AI|BehaviorTree|FinishExecute false)
    (else
      (Default|Pitch (Variables|Default|GetAirplane) -2.0))))