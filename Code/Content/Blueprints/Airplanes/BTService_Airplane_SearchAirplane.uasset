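; Behavior Tree service that picks another airplane as the target for an AI-controlled airplane.
; On search start it runs a pawn sphere overlap around the controlled pawn, sized by a Blackboard radius, filtered to B_Airplane and ignoring itself.
; Each hit overwrites the Target key, so the last result wins rather than the nearest, and an empty result leaves Target unchanged.
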(event EventReceiveSearchStart
  (params (OwnerActor :type Actor%20Object%20Reference))
  (bind _returnvalue (AI|GetAIController OwnerActor))
  (bind _outactors (Class|KismetSystemLibrary|SphereOverlapActorsNEW (Transformation|GetActorLocation (Pawn|GetControlledPawn _returnvalue)) (Class|BTFunctionLibrary|GetBlackboardValueasFloat (Variables|Default|Getradius)) (Utilities|Array|MakeArray "ObjectTypeQuery3") "/Game/Blueprints/Airplanes/B_Airplane.B_Airplane_C" (Utilities|Array|MakeArray (Pawn|GetControlledPawn _returnvalue))))
  (for _array_element _outactors
    (Class|BTFunctionLibrary|SetBlackboardValueasObject (Variables|GetTarget) _array_element)))