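; Behavior tree task that makes an AI-controlled B_Airplane fly an evasion maneuver through randomized waypoints.
; On execute, it chains points by stepping a fixed distance along random directions in a cone around the plane's starting forward vector.
; Tick steers toward the current point via SetRotationSpeed, advances within the judgement distance, and finishes successfully after the last.
; Debug spheres show path and plane; the blackboard target is stored but unused here.
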(event EventTick
  (params (OwnerActor :type Actor%20Object%20Reference) (DeltaSeconds :type Float%20%28single-precision%29))
  (if (< (Math|Float|Square (Variables|Default|GetJudgementDistance)) (Math|Vector|VectorLengthSquared (- (Variables|Default|GetCurrentEvasionPoint) (Transformation|GetActorLocation (Variables|Default|GetAirplane)))))
    (bind _relativevector (CallFunction|GetRelativeVectorwithPos (Variables|Default|GetCurrentEvasionPoint) (Variables|Default|GetAirplane) :!label _label))
    (CallFunction|SetRotationSpeed _relativevector (Variables|Default|GetAirplane))
    (Rendering|Debug|DrawDebugSphere (Transformation|GetActorLocation (Variables|Default|GetAirplane)) 1e+02 12 "(R=1.000000,G=0.000000,B=0.000000,A=1.000000)" 0.0)
    (elif (> (Utilities|Array|Length (Variables|Default|GetEvasionPoint)) (Variables|Default|GetCurrentIndex))
      (Variables|Default|SetCurrentEvasionPoint (Utilities|Array|Get(acopy) (Variables|Default|GetEvasionPoint) (Variables|Default|GetCurrentIndex)))
      (Variables|Default|SetCurrentIndex (+ (Variables|Default|GetCurrentIndex) 1))
      (goto _label)
      (else
        (AI|BehaviorTree|FinishExecute true)))))

(event EventReceiveExecute
  (params (OwnerActor :type Actor%20Object%20Reference))
  (bind _ascontroller (Utilities|Casting|CastToController OwnerActor))
  (bind _asb_airplane (Utilities|Casting|CastToB_Airplane (Pawn|GetControlledPawn _ascontroller)))
  (Variables|Default|SetAirplane _asb_airplane)
  (Variables|Default|SetTarget (AI|BehaviorTree|GetBlackboardValueasActor (Variables|Default|GetTargetKey)))
  (CallFunction|SetEvasionPoint))

(fn SetEvasionPoint
  (Variables|Default|SetCurrentIndex 0)
  (bind _output_get (Variables|Default|SetCurrentEvasionPoint (Transformation|GetActorLocation (Variables|Default|GetAirplane))))
  (LocalVariables|SetSingleEvasionPoint _output_get)
  (for _index (range 1 (Variables|Default|GetCount))
    (bind _output_get_2 (LocalVariables|SetSingleEvasionPoint (+ (* (Class|KismetMathLibrary|RandomUnitVectorinCone (Transformation|GetActorForwardVector (Variables|Default|GetAirplane)) (Math|Trig|DegreesToRadians (Variables|Default|GetOffsetAngle))) (Variables|Default|GetEvasionDistance)) (LocalVariables|GetSingleEvasionPoint))))
    (Rendering|Debug|DrawDebugSphere _output_get_2 5e+01 12 "(R=1.000000,G=0.500000,B=0.500000,A=1.000000)" 15.0)
    (Utilities|Array|Add (LocalVariables|GetLocalEvasionPoint) _output_get_2))
  (Variables|Default|SetEvasionPoint (LocalVariables|GetLocalEvasionPoint)))