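; Behavior tree decorator for airplane AI that passes when the blackboard target lies inside the pawn's forward view cone.
; It compares the angle between the pawn's forward vector and the direction to the target, via dot product and arccosine, against ViewAngle.
; Only angle is tested, with no distance or line-of-sight check.
; A passing check also draws a temporary green debug line and sphere at the target.
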(fn PerformConditionCheckAI
  (params (OwnerController :type AI%20Controller%20Object%20Reference) (ControlledPawn :type Pawn%20Object%20Reference))
  (bind _returnvalue (Transformation|GetActorForwardVector ControlledPawn))
  (bind _returnvalue_2 (Transformation|GetActorLocation ControlledPawn))
  (bind _targetkey (Variables|Default|GetTargetKey))
  (bind _viewangle (Variables|Default|GetViewAngle))
  (bind _returnvalue_3 (AI|BehaviorTree|GetBlackboardValueasActor _targetkey))
  (bind _returnvalue_4 (Transformation|GetActorLocation _returnvalue_3))
  (bind _returnvalue_5 (- _returnvalue_4 _returnvalue_2))
  (bind _returnvalue_6 (Math|Vector|Normalize _returnvalue_5))
  (bind _returnvalue_7 (Math|Vector|DotProduct _returnvalue_6 _returnvalue))
  (bind _returnvalue_8 (Class|KismetMathLibrary|DegAcos _returnvalue_7))
  (bind _returnvalue_9 (< _returnvalue_8 _viewangle))
  (if _returnvalue_9
    (Rendering|Debug|DrawDebugLine _returnvalue_2 _returnvalue_4 "(R=0.000000,G=1.000000,B=0.000000,A=1.000000)" 5.0 1e+01)
    (Rendering|Debug|DrawDebugSphere _returnvalue_4 5e+01 12 "(R=0.000000,G=1.000000,B=0.000000,A=1.000000)" 5.0))
  (return _returnvalue_9))