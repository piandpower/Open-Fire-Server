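; Blueprint function library of steering helpers that turn an airplane toward a target.
; It converts the target position into the plane's local space, and a separate check tests whether a target lies within a view angle.
; Steering rolls at full input until lateral offset is within a small dead band, zeroing pitch and yaw meanwhile.
; Once stable, it applies full pitch and yaw toward the target, scaled down when nearly aligned.
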(fn GetRelativeVector
  (params (TargetActor :type Actor%20Object%20Reference) (Airplane :type Actor%20Object%20Reference))
  (bind _relativevector (CallFunction|GetRelativeVectorwithPos (Transformation|GetActorLocation TargetActor) Airplane))
  (return _relativevector))

(fn SetRotationSpeed
  (params (TargetRelativeVector :type Vector :default "0, 0, 0") (TargetRelativeRotator :type Rotator :default "0, 0, 0") (Airplane :type B%20Airplane%20Object%20Reference))
  (bind _stableroll (CallFunction|SetRoll TargetRelativeVector Airplane))
  (if _stableroll
    (CallFunction|SetPitch TargetRelativeVector Airplane)
    (CallFunction|SetYaw TargetRelativeVector Airplane)))

(fn SetRoll
  (params (TargetRelativeVector :type Vector :default "0, 0, 0") (Airplane :type B%20Airplane%20Object%20Reference))
  (bind _y (Math|Vector|BreakVector TargetRelativeVector))
  (bind _returnvalue (Math|Float|Absolute(Float) _y))
  (if (Math|Float|InRange(Float) _y -5e+01 5e+01)
    (LocalVariables|SetStable true)
    (LocalVariables|SetRoll 0.0)
    (if (Math|Float|InRange(Float) _returnvalue 5e+01 5.5e+02)
      (LocalVariables|SetRoll (* (LocalVariables|GetRoll) (* (- _returnvalue 5e+01) 0.002))))
    (else
      (LocalVariables|SetStable false)
      (Default|Pitch Airplane 0.0)
      (Default|Yaw Airplane 0.0)
      (if (> _y 0.0)
        (LocalVariables|SetRoll 1.0)
        (else
          (LocalVariables|SetRoll -1.0)))))
  (Default|Roll Airplane (LocalVariables|GetRoll))
  (return (LocalVariables|GetStable)))

(fn SetPitch
  (params (TargetRelativeVector :type Vector :default "0, 0, 0") (Airplane :type B%20Airplane%20Object%20Reference))
  (bind (_x _y _z) (Math|Vector|BreakVector TargetRelativeVector))
  (if (> _x 0.0)
    (if (> _z 0.0)
      (LocalVariables|SetPitch -1.0 :!label _label)
      (else
        (LocalVariables|SetPitch 1.0 :!label _label_2)))
    (elif false
      (goto _label_2)
      (else
        (goto _label))))
  (if (< (Math|Float|Absolute(Float) (.Pitch (Class|KismetMathLibrary|BreakRot (Math|Rotator|FindLookatRotation (Math|Vector|MakeVector 0.0 0.0 0.0) TargetRelativeVector)))) 1e+01)
    (LocalVariables|SetPitch (* (LocalVariables|GetPitch) 0.1)))
  (Default|Pitch Airplane (LocalVariables|GetPitch)))

(fn SetYaw
  (params (TargetRelativeVector :type Vector :default "0, 0, 0") (Airplane :type B%20Airplane%20Object%20Reference))
  (if (< (.Y (Math|Vector|BreakVector TargetRelativeVector)) 0.0)
    (LocalVariables|SetYaw -1.0)
    (else
      (LocalVariables|SetYaw 1.0)))
  (if (< (Math|Float|Absolute(Float) (.Yaw (Class|KismetMathLibrary|BreakRot (Math|Rotator|FindLookatRotation (Math|Vector|MakeVector 0.0 0.0 0.0) TargetRelativeVector)))) 1e+01)
    (LocalVariables|SetYaw (* (LocalVariables|GetYaw) 0.1)))
  (Default|Yaw Airplane (LocalVariables|GetYaw)))

(fn IsView
  (params (Airplane :type B%20Airplane%20Object%20Reference) (Target :type Actor%20Object%20Reference) (ViewAngle :type Float%20%28single-precision%29 :default 0.0))
  (return (< (Math|Trig|RadiansToDegrees (Math|Trig|Acos(Degrees) (Math|Vector|DotProduct (Transformation|GetActorForwardVector Airplane) (Math|Vector|Normalize (- (Transformation|GetActorLocation Target) (Transformation|GetActorLocation Airplane)))))) ViewAngle)))

(fn GetRelativeVectorwithPos
  (params (TargetPos :type Vector :default "0, 0, 0") (Airplane :type Actor%20Object%20Reference))
  (return (Math|Vector|UnrotateVector (- TargetPos (Transformation|GetActorLocation Airplane)) (Transformation|GetActorRotation Airplane))))

(fn GetRelativeRotatorandVector
  (params (TargetActor :type Actor%20Object%20Reference) (Airplane :type Actor%20Object%20Reference))
  (bind _relativevector (CallFunction|GetRelativeVector TargetActor Airplane))
  (return (Math|Rotator|FindLookatRotation (Math|Vector|MakeVector 0.0 0.0 0.0) _relativevector) _relativevector))