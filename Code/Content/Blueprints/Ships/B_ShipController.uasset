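; B_ShipController is an AI controller that runs the BT_Ship behavior tree and turns its ship in relation to a Target.
; Its construction script starts the tree and caches the controlled pawn as a B_Ship.
; Each tick, while Target is valid, it combines the look-at rotation with the negated ship rotation.
; It passes whether that yaw is below 180 degrees to Ship.Rotate as a boolean.
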(event EventTick
  (params (DeltaSeconds :type Float%20%28single-precision%29))
  (bind _ship (Variables|Default|GetShip))
  (Utilities|IsValid (Variables|Default|GetTarget)
    (:Is%20Valid
      (Default|Rotate (Variables|Default|GetShip) (< (.Yaw (Class|KismetMathLibrary|BreakRot (Math|Rotator|CombineRotators (Math|Rotator|FindLookatRotation (Transformation|GetActorLocation _ship) (Transformation|GetActorLocation (Variables|Default|GetTarget))) (* (Transformation|GetActorRotation _ship) -1.0)))) 1.8e+02)))))

(fn ConstructionScript
  (AI|RunBehaviorTree "/Game/Blueprints/Ships/BT_Ship.BT_Ship")
  (bind _asb_ship (Utilities|Casting|CastToB_Ship (Pawn|GetControlledPawn)))
  (Variables|Default|SetShip _asb_ship))