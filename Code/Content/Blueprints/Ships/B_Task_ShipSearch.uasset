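; Behavior tree task that finds a target for an AI-controlled B_Ship.
; It runs a sphere overlap around the ship using that ship's SearchRange and TargetObjectType, filtered to B_Component actors.
; Each hit is written to the Target blackboard key and calls FinishExecute with success, without breaking the loop.
; Failed casts or an empty result never call FinishExecute.
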(event EventReceiveExecute
  (params (OwnerActor :type Actor%20Object%20Reference))
  (bind _ascontroller (Utilities|Casting|CastToController OwnerActor))
  (bind _asb_ship (Utilities|Casting|CastToB_Ship (Pawn|GetControlledPawn _ascontroller)))
  (Utilities|IsValid _asb_ship
    (:Is%20Valid
      (bind _outactors (Class|KismetSystemLibrary|SphereOverlapActorsNEW (Transformation|GetActorLocation _asb_ship) (Variables|/Game/Blueprints/Ships/B_Ship.B_Ship_C|GetSearchRange _asb_ship) (Variables|/Game/Blueprints/Ships/B_Ship.B_Ship_C|GetTargetObjectType _asb_ship) "/Game/Blueprints/Components/B_Component.B_Component_C"))
      (for _array_element _outactors
        (AI|Components|Blackboard|SetValueasObject (Class|BTFunctionLibrary|GetOwnersBlackboard) (Utilities|Name|MakeLiteralName "Target") _array_element)
        (AI|BehaviorTree|FinishExecute true)))))