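; Ship actor that moves and turns on start/stop commands and carries AI-driven cannons.
; Tick integrates speed and yaw rate with acceleration and limits, moving without sweep; forward speed decelerates when stopped, but yaw rate persists after RotateStop.
; Intialize sets mesh and collision channel, then spawns and attaches a B_Cannon running BT_Weapon at each arrow component, passing on the channel.
; BeginPlay clears the blackboard Target.
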(event EventTick
  (params (DeltaSeconds :type Float%20%28single-precision%29))
  (bind _returnvalue (Transformation|GetActorRotation))
  (bind _maxrotatespeed (Variables|Default|GetMaxRotateSpeed))
  (bind (_pitch _yaw _roll) (Class|KismetMathLibrary|BreakRot _returnvalue))
  ;[1 1 1] Move Forward
  (if (Variables|Default|GetIsMoveForward)
    (Variables|Default|SetCurSpeed (Math|Float|Min(Float) (+ (Variables|Default|GetCurSpeed) (* DeltaSeconds (Variables|Default|GetAcceleration))) (Variables|Default|GetMaxSpeed)))
    (else
      (Variables|Default|SetCurSpeed (Math|Float|Max(Float) (- (Variables|Default|GetCurSpeed) (* DeltaSeconds (Variables|Default|GetDeceleration))) 0.0))))
  (Transformation|SetActorLocation (+ (* (Transformation|GetActorForwardVector) (* (Variables|Default|GetCurSpeed) DeltaSeconds)) (Transformation|GetActorLocation)) false)
  ;[1 1 1] Rotate
  (Variables|Default|SetCurRotateSpeed (Math|Float|Clamp(Float) (+ (Variables|Default|GetCurRotateSpeed) (* DeltaSeconds (Variables|Default|GetRotateToRightDesire) (Variables|Default|GetAngularAcceleration))) (- 0.0 _maxrotatespeed) _maxrotatespeed))
  (Transformation|SetActorRotation (Class|KismetMathLibrary|MakeRot _pitch (+ _yaw (* (Variables|Default|GetCurRotateSpeed) DeltaSeconds)) _roll)))

(event EventBeginPlay
  (AI|Components|Blackboard|SetValueasObject (AI|GetBlackboard self) (Utilities|Name|MakeLiteralName "Target") 0))

(fn ConstructionScript)

(fn MoveForward
  (Variables|Default|SetIsMoveForward true))

(fn Rotate
  (params (IsRight :type Boolean))
  (if IsRight
    (Variables|Default|SetRotateToRightDesire 1.0)
    (else
      (Variables|Default|SetRotateToRightDesire -1.0))))

(fn MoveStop
  (Variables|Default|SetIsMoveForward false))

(fn RotateStop
  (Variables|Default|SetRotateToRightDesire 0.0))

(fn Intialize
  (params (StaticMesh :type Static%20Mesh%20Object%20Reference) (CollisionChannel :type ECollisionChannel%20Enum :default "ECC_WorldStatic"))
  (Components|StaticMesh|SetStaticMesh (Variables|Default|GetStaticMesh) StaticMesh)
  (Collision|SetCollisionObjectType (Variables|Default|GetSphere) CollisionChannel)
  (for _array_element (Variables|Default|GetArrayComponentArrow)
    (bind _returnvalue (AI|SpawnAIFromClass "/Game/Blueprints/Components/Weapons/Cannons/B_Cannon.B_Cannon_C" "/Game/Blueprints/Components/Weapons/BT_Weapon.BT_Weapon" "0, 0, 0" "0, 0, 0" false))
    (bind _asb_weapon (Utilities|Casting|CastToB_Weapon _returnvalue))
    (Default|Initialize _asb_weapon CollisionChannel)
    (Class|SceneComponent|Attachto _asb_weapon _array_element "None" "KeepRelativeOffset" true)))