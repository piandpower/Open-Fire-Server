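; B_ShipFactory is an actor that spawns two AI-controlled Lettow-Vorbeck Class A ships when play begins.
; Both spawn at fixed X offsets from the factory running BT_Ship, and each is initialized as a B_Ship on its own collision channel with zeroed ship data.
; Component creation looks unfinished: CreateComponent is an empty stub, and neither its call nor the component-data loop is on an executed path.
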(event EventBeginPlay
  (bind _returnvalue (AI|SpawnAIFromClass "/Game/Blueprints/Ships/Frigates/B_LettowVorbeckClassA.B_LettowVorbeckClassA_C" "/Game/Blueprints/Ships/BT_Ship.BT_Ship" (+ (Transformation|GetActorLocation) "100.000000, 0, 0") "0, 0, 0" false))
  (bind _asb_ship (Utilities|Casting|CastToB_Ship _returnvalue))
  (Default|Intialize _asb_ship "ECC_GameTraceChannel1" (Utilities|Struct|MakeShipDataTable) (Utilities|Array|MakeArray 0))
  (bind _returnvalue_2 (AI|SpawnAIFromClass "/Game/Blueprints/Ships/Frigates/B_LettowVorbeckClassA.B_LettowVorbeckClassA_C" "/Game/Blueprints/Ships/BT_Ship.BT_Ship" (+ (Transformation|GetActorLocation) "-2000.000000, 0, 0") "0, 0, 0" false))
  (bind _asb_ship_2 (Utilities|Casting|CastToB_Ship _returnvalue_2))
  (Default|Intialize _asb_ship_2 "ECC_GameTraceChannel2" (Utilities|Struct|MakeShipDataTable) (Utilities|Array|MakeArray (stale _newparam1))))

(fn ConstructionScript)

(fn CreateComponent
  (params (NewParam :type Ship%20Component%20Data%20Table%20Structure))
  (return 0))