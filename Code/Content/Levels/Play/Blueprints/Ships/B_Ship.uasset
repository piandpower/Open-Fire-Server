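; Ship Blueprint that handles forward propulsion, turning and mounting of ship components.
; While moving forward, Tick applies constant forward force and eases a clamped turn desire toward right or left, integrating it into capped yaw speed and rotation.
; Move and rotate functions set the flags or reset turn desire.
; Intialize initializes supplied components and attaches each to its matching arrow by array index.
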(event EventTick
  (params (DeltaSeconds :type Float%20%28single-precision%29))
  (bind _returnvalue (Transformation|GetActorRotation))
  (bind _maxrotatespeed (Variables|Default|GetMaxRotateSpeed))
  (bind (_pitch _yaw _roll) (Class|KismetMathLibrary|BreakRot _returnvalue))
  ;[1 1 1] Move Forward
  (if (Variables|Default|GetIsMoveForward)
    (Physics|AddForce self (* (Transformation|GetActorForwardVector) (Math|Float|MakeLiteralFloat 1e+03)) "None")
    ;[1 1 1] Rotate
    (if (Variables|Default|GetIsRotateRight)
      (Variables|Default|SetRotateToRightDesire (Math|Float|Clamp(Float) (+ (Variables|Default|GetRotateToRightDesire) DeltaSeconds) -1.0))
      (else
        (bind _output_get (Variables|Default|SetRotateToRightDesire (Math|Float|Clamp(Float) (- (Variables|Default|GetRotateToRightDesire) DeltaSeconds) -1.0)))))
    (Variables|Default|SetCurRotateSpeed (Math|Float|Clamp(Float) (+ (Variables|Default|GetCurRotateSpeed) (* DeltaSeconds _output_get (Variables|Default|GetAngularAcceleration))) (- 0.0 _maxrotatespeed) _maxrotatespeed))
    (Transformation|SetActorRotation (Class|KismetMathLibrary|MakeRot _pitch (+ _yaw (* (Variables|Default|GetCurRotateSpeed) DeltaSeconds)) _roll))))

(fn ConstructionScript)

(fn MoveForward
  (Variables|Default|SetIsMoveForward true))

(fn Rotate
  (params (IsRight :type Boolean))
  (if IsRight
    (Variables|Default|SetIsRotateRight true)
    (else
      (Variables|Default|SetIsRotateRight false))))

(fn MoveStop
  (Variables|Default|SetIsMoveForward false))

(fn RotateStop
  (Variables|Default|SetRotateToRightDesire 0.0))

(fn Intialize
  (params (ShipData :type Ship%20Data%20Structure) (Component :type Array%20of%20B%20Component%20Object%20References))
  (for (_array_element _array_index) (Variables|Default|GetArrayComponentArrow)
    (Default|Initialize (Utilities|Array|Get(acopy) Component _array_index))
    (Class|SceneComponent|Attachto (Utilities|Array|Get(acopy) Component _array_index) _array_element "None" "KeepRelativeOffset" true)))