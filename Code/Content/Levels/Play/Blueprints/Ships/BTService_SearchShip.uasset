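; A behavior tree service that finds nearby ships for an AI-controlled ship.
; On search start, it runs a pawn sphere overlap around the controlled B_Ship using its SearchRange, filtered to B_Ship and ignoring itself.
; Each hit is written to the Target blackboard key in turn, so the last ship in the result becomes the target, with no distance or team check.
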(event EventReceiveSearchStart
  (params (OwnerActor :type Actor%20Object%20Reference))
  (bind _ascontroller (Utilities|Casting|CastToController OwnerActor))
  (bind _asb_ship (Utilities|Casting|CastToB_Ship (Pawn|GetControlledPawn _ascontroller)))
  (bind _outactors (Class|KismetSystemLibrary|SphereOverlapActorsNEW (Transformation|GetActorLocation _asb_ship) (Variables|/Game/Levels/Play/Blueprints/Ships/B_Ship.B_Ship_C|GetSearchRange _asb_ship) (Utilities|Array|MakeArray "ObjectTypeQuery3") "/Game/Levels/Play/Blueprints/Ships/B_Ship.B_Ship_C" (Utilities|Array|MakeArray (Pawn|GetControlledPawn _ascontroller))))
  (for _array_element _outactors
    (Class|BTFunctionLibrary|SetBlackboardValueasObject (Variables|Default|GetTarget) _array_element)))