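; Behavior tree task that steers an AI-controlled B_Ship toward the actor in its Target blackboard key.
; On execute it caches the controller's pawn as the ship.
; Each tick it turns the ship left or right by the sign of the yaw difference to the target, then moves it forward.
; It has no arrival check and never calls Finish Execute.
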(event EventTick
  (params (OwnerActor :type Actor%20Object%20Reference) (DeltaSeconds :type Float%20%28single-precision%29))
  (bind _ship (Variables|Default|GetShip))
  (bind _ship_2 (Variables|Default|GetShip))
  (Default|Rotate _ship (< (.Yaw (Class|KismetMathLibrary|BreakRot (Math|Rotator|Delta(Rotator) (Transformation|GetActorRotation _ship_2) (Math|Rotator|FindLookatRotation (Transformation|GetActorLocation _ship_2) (Transformation|GetActorLocation (AI|BehaviorTree|GetBlackboardValueasActor (Variables|Default|GetTarget))))))) 0.0))
  (Default|MoveForward _ship))

(event EventReceiveExecute
  (params (OwnerActor :type Actor%20Object%20Reference))
  (bind _ascontroller (Utilities|Casting|CastToController OwnerActor))
  (bind _asb_ship (Utilities|Casting|CastToB_Ship (Pawn|GetControlledPawn _ascontroller)))
  (Variables|Default|SetShip _asb_ship))