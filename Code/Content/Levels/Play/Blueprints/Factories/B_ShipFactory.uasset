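; B_ShipFactory is a factory that spawns a test fleet of AI-driven ships with components at BeginPlay.
; Each TestFleetData entry sets a transform for SpawnShip, which spawns a B_LettowVorbeckClassA running BT_Ship.
; CreateComponent spawns a B_Cannon pawn running BT_Weapon per component entry, and the collected components go to the ship's Intialize.
; Classes are hard-coded; name, team and component data contents are unused.
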(event EventBeginPlay
  (bind _returnvalue (Utilities|Name|MakeLiteralName "None"))
  (for _array_element (Variables|Default|GetTestFleetData)
    (CallFunction|SpawnShip _returnvalue (Variables|Default|GetTestCompnentData) (Math|Vector|MakeVector (.posX (Utilities|Struct|BreakFleetData _array_element)) (.posY (Utilities|Struct|BreakFleetData _array_element)) (.posZ (Utilities|Struct|BreakFleetData _array_element))) (Class|KismetMathLibrary|MakeRot (.rotX (Utilities|Struct|BreakFleetData _array_element)) (.rotY (Utilities|Struct|BreakFleetData _array_element)) (.rotZ (Utilities|Struct|BreakFleetData _array_element))) _returnvalue)))

(fn ConstructionScript)

(fn CreateComponent
  (params (NewParam :type Component%20Data%20Structure))
  (bind _returnvalue (AI|SpawnAIFromClass "/Game/Levels/Play/Blueprints/Components/Weapons/Cannons/B_Cannon.B_Cannon_C" "/Game/Levels/Play/Blueprints/Components/Weapons/BT_Weapon.BT_Weapon" "0, 0, 0" "0, 0, 0" false))
  (bind _asb_component (Utilities|Casting|CastToB_Component _returnvalue))
  (return _asb_component))

(fn SpawnShip
  (params (Name :type Name%20%28by%20ref%29) (Components :type Array%20of%20Component%20Data%20Structures) (Location :type Vector%20%28by%20ref%29 :default "0, 0, 0") (Rotation :type Rotator%20%28by%20ref%29 :default "0, 0, 0") (Team :type Name%20%28by%20ref%29))
  (bind _returnvalue (AI|SpawnAIFromClass "/Game/Levels/Play/Blueprints/Ships/Frigates/B_LettowVorbeckClassA.B_LettowVorbeckClassA_C" "/Game/Levels/Play/Blueprints/Ships/BT_Ship.BT_Ship" Location Rotation false))
  (bind _asb_ship (Utilities|Casting|CastToB_Ship _returnvalue))
  (for _array_element Components
    (bind _newparam1 (CallFunction|CreateComponent _array_element))
    (Utilities|Array|AppendArray (Variables|Default|GetCreatedComponent) (Utilities|Array|MakeArray _newparam1)))
  (Default|Intialize :self _asb_ship :Component (Variables|Default|GetCreatedComponent))
  (Utilities|Array|Clear (Variables|Default|GetCreatedComponent)))