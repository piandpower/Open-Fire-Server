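; OpenFirePawn is a camera pawn that orbits a selected target and creates the OpenFireHUD widget on BeginPlay, passing itself to it.
; Each Tick it sits at a set distance from the target along the camera rotator's forward vector, facing the target.
; RotateCamera adjusts that rotator with clamped pitch, and SetCurrentTarget cycles through the Targets array with wraparound.
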(event EventBeginPlay
  (bind _returnvalue (UserInterface|CreateWidget "/Game/Levels/Play/Blueprints/GameMode/OpenFireHUD.OpenFireHUD_C"))
  (Default|SetPawn _returnvalue self)
  (UserInterface|Viewport|AddtoViewport _returnvalue 0))

(event EventActorBeginOverlap
  (params (OtherActor :type Actor%20Object%20Reference)))

(event EventTick
  (params (DeltaSeconds :type Float%20%28single-precision%29))
  (bind _cameradistance (Variables|Default|GetCameraDistance))
  (bind _target (Variables|Default|GetTarget))
  (bind _camerarotator (Variables|Default|GetCameraRotator))
  (bind _returnvalue (Transformation|GetActorLocation _target))
  (bind _returnvalue_2 (Math|Vector|GetForwardVector _camerarotator))
  (bind _returnvalue_3 (* _returnvalue_2 _cameradistance))
  (bind _returnvalue_4 (+ _returnvalue_3 _returnvalue))
  (Utilities|IsValid (Variables|Default|GetTarget)
    (:Is%20Valid
      (Transformation|SetActorLocation _returnvalue_4 false)
      (Transformation|SetActorRotation (Math|Rotator|FindLookatRotation _returnvalue_4 _returnvalue)))))

(fn ConstructionScript)

(fn SetCurrentTarget
  (if (!= (Utilities|Array|Length (Variables|Default|GetTargets)) 0)
    (if (>= (Utilities|Array|LastIndex (Variables|Default|GetTargets)) (+ (Variables|Default|GetTargetIndex) 1))
      (bind _output_get (Variables|Default|SetTargetIndex (+ (Variables|Default|GetTargetIndex) 1)))
      (else
        (Variables|Default|SetTargetIndex 0)))
    (Variables|Default|SetTarget (Utilities|Array|Get(acopy) (Variables|Default|GetTargets) _output_get))))

(fn RotateCamera
  (params (Yaw :type Float%20%28single-precision%29 :default 0.0) (Pitch :type Float%20%28single-precision%29 :default 0.0))
  (Variables|Default|SetCameraRotator (Class|KismetMathLibrary|MakeRot (Math|Float|Clamp(Float) (+ Pitch (.Pitch (Class|KismetMathLibrary|BreakRot (Variables|Default|GetCameraRotator)))) -89.0 89.0) (+ Yaw (.Yaw (Class|KismetMathLibrary|BreakRot (Variables|Default|GetCameraRotator)))) (.Roll (Class|KismetMathLibrary|BreakRot (Variables|Default|GetCameraRotator))))))