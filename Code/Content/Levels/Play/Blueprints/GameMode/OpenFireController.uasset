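; Player controller for the open-fire pawn, handling targeting and camera input.
; On BeginPlay it caches the controlled pawn, then after a short delay passes all B_Ship actors to it as targets.
; Releasing Space calls the pawn's SetCurrentTarget.
; Dragging one tracked finger rotates the pawn's camera, with movement normalized by viewport size so a full-screen swipe equals a full turn.
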(event EventBeginPlay
  (bind _asopen_fire_pawn (Utilities|Casting|CastToOpenFirePawn (Pawn|GetControlledPawn)))
  (Variables|Default|SetOpenFirePawn _asopen_fire_pawn)
  (Utilities|FlowControl|Delay 0.2)
  (bind _outactors (Actor|GetAllActorsOfClass "/Game/Levels/Play/Blueprints/Ships/B_Ship.B_Ship_C"))
  (Variables|/Game/Levels/Play/Blueprints/GameMode/OpenFirePawn.OpenFirePawn_C|SetTargets (Variables|Default|GetOpenFirePawn) _outactors))

(event Input|KeyboardEvents|SpaceBar
  (:Released
    (Default|SetCurrentTarget (Variables|Default|GetOpenFirePawn))))

(event Input|TouchEvents|InputTouch
  (params (Location :type Vector :default "0, 0, 0") (FingerIndex :type ETouchIndex%20Enum :default "Touch1"))
  (bind (_sizex _sizey) (HUD|GetViewportSize))
  (:Moved
    (if (and (Variables|Default|GetDragged) (== FingerIndex (Variables|Default|GetTouchIndex)))
      (Default|RotateCamera (Variables|Default|GetOpenFirePawn) (* (/ (.X (Math|Vector|BreakVector (- Location (Variables|Default|GetLastLocation)))) (Math|Conversions|ToFloat(Integer) _sizex)) 3.6e+02) (* (/ (.Y (Math|Vector|BreakVector (- Location (Variables|Default|GetLastLocation)))) (Math|Conversions|ToFloat(Integer) _sizey)) 3.6e+02))
      (Variables|Default|SetLastLocation Location))))

(event Input|TouchEvents|InputTouch
  (params (Location :type Vector :default "0, 0, 0") (FingerIndex :type ETouchIndex%20Enum :default "Touch1"))
  (:Pressed
    (Variables|Default|SetDragged true)
    (Variables|Default|SetLastLocation Location)
    (Variables|Default|SetTouchIndex FingerIndex))
  (:Released
    (Variables|Default|SetDragged false)))

(fn ConstructionScript)