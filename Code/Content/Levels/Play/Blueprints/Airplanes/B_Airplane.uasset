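; Physics-driven airplane with an AI blackboard, which receives its search radius and view angle on BeginPlay.
; Move, Roll, Pitch and Yaw store power inputs that Tick turns into motion on the physics body.
; Thrust is a mass-scaled forward force, applied only while forward-axis speed is below the maximum.
; Angular velocity is set directly from the rotation inputs, with roll inverted, and rotated from local to world space.
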(event EventBeginPlay
  (AI|Components|Blackboard|SetValueasFloat (AI|GetBlackboard self) (Utilities|Name|MakeLiteralName "SearchRadius") (Variables|Default|GetSearchRadius))
  (AI|Components|Blackboard|SetValueasFloat (AI|GetBlackboard self) (Utilities|Name|MakeLiteralName "ViewAngle") (Variables|Default|GetViewAngle)))

(event EventTick
  (params (DeltaSeconds :type Float%20%28single-precision%29))
  (CallFunction|SetLinearVelocity)
  (CallFunction|SetAngularVelocity))

(fn ConstructionScript)

(fn Move
  (params (Desire :type Float%20%28single-precision%29 :default 0.0))
  (Variables|Components|SetForwardPower Desire))

(fn Roll
  (params (Desire :type Float%20%28single-precision%29 :default 0.0))
  (Variables|Default|SetRollPower Desire))

(fn Pitch
  (params (Desire :type Float%20%28single-precision%29 :default 0.0))
  (Variables|Default|SetPitchPower Desire))

(fn Yaw
  (params (Desire :type Float%20%28single-precision%29 :default 0.0))
  (Variables|Default|SetYawPower Desire))

(fn CalculateRotSpeed
  (params (CurrentSpeed :type Float%20%28single-precision%29 :default 0.0) (DesireSpeed :type Float%20%28single-precision%29 :default 0.0) (MaxSpeed :type Float%20%28single-precision%29 :default 0.0))
  (if (Math|Float|InRange(Float) CurrentSpeed (- 0.0 MaxSpeed) MaxSpeed)
    (return DesireSpeed)))

(fn SetAngularVelocity
  (bind _rollspeed (Variables|Default|GetRollSpeed))
  (bind _ptichspeed (Variables|Default|GetPtichSpeed))
  (bind _returnvalue (Class|PrimitiveComponent|GetPhysicsAngularVelocity "None"))
  (LocalVariables|SetLocalRoll (.X (Math|Vector|BreakVector _returnvalue)))
  (LocalVariables|SetLocalPitch (.Y (Math|Vector|BreakVector _returnvalue)))
  (LocalVariables|SetLocalYaw (.Z (Math|Vector|BreakVector _returnvalue)))
  (if (Math|Float|InRange(Float) (LocalVariables|GetLocalRoll) (- 0.0 _rollspeed) _rollspeed)
    _
    (else
      _))
  (LocalVariables|SetLocalRoll (- 0.0 (* (Variables|Default|GetRollSpeed) (Variables|Default|GetRollPower))))
  (if (Math|Float|InRange(Float) (LocalVariables|GetLocalPitch) (- 0.0 _ptichspeed) _ptichspeed)
    _
    (else
      _))
  (LocalVariables|SetLocalPitch (* (Variables|Default|GetPtichSpeed) (Variables|Default|GetPitchPower)))
  (LocalVariables|SetLocalYaw (* (Variables|Default|GetYawSpeed) (Variables|Default|GetYawPower)))
  (Class|PrimitiveComponent|SetPhysicsAngularVelocity (Math|Vector|RotateVector (Math|Vector|MakeVector (LocalVariables|GetLocalRoll) (LocalVariables|GetLocalPitch) (LocalVariables|GetLocalYaw)) (Transformation|GetActorRotation)) false "None"))

(fn SetLinearVelocity
  (bind _staticmesh (Variables|Default|GetStaticMesh))
  (bind _returnvalue (Math|Vector|GetForwardVector _staticmesh))
  (if (< (Math|Vector|VectorLengthSquared (Math|Vector|ProjectVectorontoVector (Transformation|GetComponentVelocity _staticmesh) _returnvalue)) (Math|Float|Square (Variables|Default|GetMaxSpeed)))
    (Physics|AddForce (* _returnvalue (* (* (Physics|GetMass _staticmesh) (Variables|Default|GetAcceleration)) (Variables|Components|GetForwardPower))) "None")))